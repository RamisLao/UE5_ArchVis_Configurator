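; Orbit camera that circles a target actor around the world Z axis in response to the player controller's horizontal look event.
; While active and rotatable, look input supplies only direction, stepping rotation by speed and delta time.
; RotateAroundTarget rotates the actor's location vector and offsets the camera by the target's location, while Tick keeps it facing the target.
; Resetting setup restores the actor location saved at BeginPlay.
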(event `self.ReceiveBeginPlay`
  (`parent.ReceiveBeginPlay`)
  (bind _asbp_kambio_player_controller (cast `/Game/Kambio/Blueprints/Player/BP_KambioPlayerController` (`GameplayStatics.GetPlayerController` 0)))
  (add `/Game/Kambio/Blueprints/Player/BP_KambioPlayerController.EventLookHorizontal` _asbp_kambio_player_controller (delegate `OnLookHorizontal`))
  (set `self.InitialPosition` (`self.K2_GetActorLocation`))
  (`self.RotateAroundTarget` 0.0))

(event `OnLookHorizontal`
  (params (Value :type "Float (double-precision)"))
  (if (`self.IsActive`)
    (if (`self.CanRotate`)
      (if (not (== Value 0.0))
        (`self.RotateAroundTarget` (`KismetMathLibrary.SelectFloat` -1.0 1.0 (< Value 0.0)))))))

(event `self.ReceiveTick`
  (params (DeltaSeconds :type "Float (single-precision)"))
  (bind _cameracomponent (`self.CameraComponent`))
  (if (`self.IsActive`)
    (`SceneComponent.K2_SetWorldRotation` _cameracomponent (`KismetMathLibrary.FindLookAtRotation` (`SceneComponent.K2_GetComponentLocation` _cameracomponent) (`self.K2_GetActorLocation` (`self.TargetActor`))) false false)))

(fn `ReturnToInitialPosition`
  (`self.K2_SetActorLocation` (`self.InitialPosition`))
  (`self.RotateAroundTarget` 0.0))

(fn `ReturnToInitialSetup`
  (`parent.ReturnToInitialSetup`)
  (`self.ReturnToInitialPosition`))

(fn `RotateAroundTarget`
  (params (AxisValue :type "Float (double-precision)"))
  (bind _returnvalue (`KismetMathLibrary.RotateAngleAxis` (`self.K2_GetActorLocation`) (* AxisValue (`self.RotationSpeed`) (`GameplayStatics.GetWorldDeltaSeconds`)) (0.0 0.0 1.0)))
  (`SceneComponent.K2_SetWorldLocation` (`self.SceneComponent`) _returnvalue false false)
  (`SceneComponent.K2_SetWorldLocation` (`self.CameraComponent`) (+ _returnvalue (`self.K2_GetActorLocation` (`self.TargetActor`))) false false))

(fn `UserConstructionScript`)