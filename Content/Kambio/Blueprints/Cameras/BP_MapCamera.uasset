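; BP_MapCamera is a map camera that hides configured static meshes from its scene capture according to the current floor tag.
; When given a new floor tag, it finds the matching floor entry in the DAConfigFloors data.
; Static mesh actors carrying that entry's ignore tags are appended to the capture component's HiddenActors.
; The list is never cleared here, so hidden actors accumulate across floor changes.
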(fn `SetIgnoreMeshesByFloorTag`
  (params (FloorTag :type String))
  (if (not (`KismetStringLibrary.EqualEqual_StrStr` FloorTag (`self.CurrentFloorTag`)))
    (bind _output_get (set `self.CurrentFloorTag` FloorTag))
    (for _array_element (`/Game/Kambio/DataAssets/PDAs/PDA_ConfigSections.FloorIdsToIgnoreInCameraMapIds` (`self.DA_ConfigFloors`))
      (if (`KismetStringLibrary.EqualEqual_StrStr` _output_get (`/Game/Kambio/DataAssets/PDAs/PDA_SectionIdToIgnoreInCameraMapIds.FloorId` _array_element))
        (for _array_element_2 (`/Game/Kambio/DataAssets/PDAs/PDA_SectionIdToIgnoreInCameraMapIds.IgnoreInCameraMapIds` _array_element)
          (bind _outactors (`GameplayStatics.GetAllActorsOfClassWithTag` "/Script/Engine.StaticMeshActor" (`KismetStringLibrary.Conv_StringToName` _array_element_2)))
          (`KismetArrayLibrary.Array_Append` (`SceneCaptureComponent.HiddenActors` (`self.CaptureComponent2D`)) _outactors))
        (break)))))

(fn `UserConstructionScript`)