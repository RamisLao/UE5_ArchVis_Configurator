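; Interactable door that swings open on Interact and closes automatically when the Kambio character leaves its box trigger.
; A single timeline lerps the Arrow component's yaw toward an open angle and reverses to close, with play rate derived from separate open and close durations.
; The construction script applies a configurable static mesh, so the Blueprint can serve different door models.
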(event `/Game/Kambio/Blueprints/I_Interactable.Interact`
  (if (not (`self.IsOpen`))
    (set `self.IsOpen` true)
    (`TimelineComponent.SetPlayRate` (`self.OpenCloseDoor`) (/ 1.0 (`self.TimeToOpen`)))
    (bind (_direction _doortrack) (`Timeline|OpenCloseDoor` :!label _label)
      (:`Update`
        (`SceneComponent.K2_SetRelativeRotation` (`self.Arrow`) (`KismetMathLibrary.MakeRotator` 0.0 0.0 (`KismetMathLibrary.Lerp` 0.0 (`self.AngleWhenOpen`) _doortrack)) false false)))))

(event `self.Box.OnComponentEndOverlap`
  (params (OverlappedComponent :type "PrimitiveComponent Object Reference") (OtherActor :type "Actor Object Reference") (OtherComp :type "PrimitiveComponent Object Reference") (OtherBodyIndex :type Integer))
  (if (`self.IsOpen`)
    (cast `/Game/Kambio/Blueprints/Player/BP_KambioCharacter` OtherActor)
    (set `self.IsOpen` false)
    (`TimelineComponent.SetPlayRate` (`self.OpenCloseDoor`) (/ 1.0 (`self.TimeToClose`)))
    (goto _label :!via `Reverse`)))

(fn `UserConstructionScript`
  (`StaticMeshComponent.SetStaticMesh` (`self.StaticMesh`) (`self.Mesh`)))