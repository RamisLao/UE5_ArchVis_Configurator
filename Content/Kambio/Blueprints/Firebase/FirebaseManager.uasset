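; FirebaseManager is a Blueprint that exercises Firebase email sign-in and database writes, apparently as an integration test with placeholder data.
; On BeginPlay it starts the sign-in, then builds a document with a string and a string array and adds it to the "users" path without waiting for the login result.
; Success and failure callbacks only print the user UID, new data ID or error message.
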(event `self.ReceiveBeginPlay`
  (`parent.ReceiveBeginPlay`)
  (`FBPAuth.FBPSignInWithEmailAndPassword` "" "" (delegate `OnLoginSuccess`) (delegate `OnLoginFail`))
  (bind _returnvalue (`FBPDataObject.FBPBeginWriteDocument`))
  (bind _returnvalue_2 (`FBPDataObject.AddString` "name" "value" _returnvalue))
  (bind _returnvalue_3 (`FBPDataObject.AddStringArray` "string array" (`|MakeArray` "1" "2" "3") _returnvalue_2))
  (`FBPRealtimeDatabase.FBPAddData` (`|MakeArray` "users") _returnvalue_3 (delegate `OnDataAdded`) (delegate `OnFailToAddData`)))

(event `OnLoginFail`
  (params (ErrorMessage :type String))
  (`KismetSystemLibrary.PrintString` ErrorMessage))

(event `OnDataAdded`
  (params (DataId :type String))
  (`KismetSystemLibrary.PrintString` DataId))

(event `OnFailToAddData`
  (params (ErrorMessage :type String))
  (`KismetSystemLibrary.PrintString` ErrorMessage))

(event `OnLoginSuccess`
  (params (FirebaseUser :type "BPFirebaseUser Structure"))
  (`KismetSystemLibrary.PrintString` FirebaseUser_Uid))

(fn `UserConstructionScript`)