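; Player controller for Kambio that runs the Configuration, Exploration and Cinematics app modes, each with its own HUD and input handling.
; Switches view targets between tagged BP_CustomCamera actors from UI panel changes or exploration clicks, hiding each camera's occluder meshes.
; Handles gated camera rotation, wheel scrolling of panels, and a map camera that follows above the active camera.
; SequenceComponent drives fades and cinematics; Pixel Streaming input is printed, and screenshots are sent as PNG bytes.
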(event `Key|LeftMouseButton`
  (params (Key :type "Key Structure"))
  ;[1 0.9141 0] Input
  (:`Pressed`
    (if (`|EnumEquality` (`self.CurrentAppMode`) "NewEnumerator1")
      (set `self.TimeSinceLeftMousePressed` 0.0)
      (elif (`self.CanActivateCameraRotation`)
        (set `self.CanRotateCamera` true))))
  (:`Released`
    (switch `/Game/Kambio/DataAssets/Config/Enums/Enum_AppMode` (`self.CurrentAppMode`)
      (:`NewEnumerator0`
        (if (`self.CanActivateCameraRotation`)
          (set `self.CanRotateCamera` false)))
      (:`NewEnumerator1`
        (if (< (`self.TimeSinceLeftMousePressed`) (`self.DelayThresholdToChangeCamera`))
          (`self.SetNewCameraForExploration`)))
      (:`NewEnumerator2`
        (`self.GoToConfigurationMode`)))))

(event `self.ReceiveBeginPlay`
  (bind _uiconfigcomponent (`self.UIConfigComponent`))
  ;[0 0.4609 1] Setup
  (`/Game/Kambio/Blueprints/Gameplay/SequenceComponent.CreateWidgetFade` (`self.SequenceComponent`) true)
  (set `self.bShowMouseCursor` true)
  (set `self.CanActivateCameraRotation` false)
  (set `self.CanRotateCamera` false)
  (bind _outactors (`GameplayStatics.GetAllActorsOfClass` "/Game/Kambio/Blueprints/Camera/BP_MapCamera.BP_MapCamera_C"))
  (set `self.MapCamera` (`|GetArrayItem` _outactors))
  (add `PixelStreamingInput.OnInputEvent` (`self.PixelStreamingInput`) (delegate `OnPixelStreamingInputEvent`))
  (add `/Game/Kambio/Blueprints/UI/Component_UIConfig.OnActiveWidgetPanelChanged` _uiconfigcomponent (delegate `OnActiveWidgetPanelChanged`))
  (add `/Game/Kambio/Blueprints/UI/Component_UIConfig.OnButtonConfigurationClicked` _uiconfigcomponent (`|CreateDelegate` :!event `GoToConfigurationMode`))
  (add `/Game/Kambio/Blueprints/UI/Component_UIConfig.OnButtonExplorationClicked` _uiconfigcomponent (`|CreateDelegate` :!event `GoToExplorationMode`))
  (add `/Game/Kambio/Blueprints/UI/Component_UIConfig.OnButtonCinematicsClicked` _uiconfigcomponent (`|CreateDelegate` :!event `GoToCinematicMode`))
  (bind _outactors_2 (`GameplayStatics.GetAllActorsOfClassWithTag` "/Game/Kambio/Blueprints/Camera/BP_CustomCamera.BP_CustomCamera_C" (`KismetStringLibrary.Conv_StringToName` (`/Game/Kambio/DataAssets/Config/PDAs/PDA_ConfigGameplay.InitCameraTagForExploration` (`self.DA_ConfigGameplay`)))))
  (`self.Set New Camera` (`|GetArrayItem` _outactors_2) false true 0.0)
  (`KismetSystemLibrary.Delay` 0.5)
  (`/Game/Kambio/Blueprints/Gameplay/SequenceComponent.FadeOut` (`self.SequenceComponent`))
  (`KismetSystemLibrary.Delay` 1.5)
  (`/Game/Kambio/Blueprints/Gameplay/SequenceComponent.DestroyWidgetFade` (`self.SequenceComponent`))
  (`self.GoToConfigurationMode`))

(event `OnPixelStreamingInputEvent`
  (params (Descriptor :type String))
  (bind (_stringvalue _success) (`PixelStreamingInput.GetJsonStringValue` (`self.PixelStreamingInput`) Descriptor ""))
  ;[0 0.4609 1] Setup
  (if _success
    (`KismetSystemLibrary.PrintString` _stringvalue)))

(event `InputAxis|LookHorizontal`
  (params (AxisValue :type "Float (single-precision)"))
  ;[1 0.9141 0] Input
  (if (`self.CanRotateCamera`)
    (`self.RotateHorizontally` AxisValue)))

(event `OnActiveWidgetPanelChanged`
  (params (ActiveSwitcherPanel :type "/Game/Kambio/Blueprints/UI/Widgets/Panels/Widget_SwitcherPanel Object Reference") (ResetCamera :type Boolean))
  (`self.SetNewCameraForConfiguration` ActiveSwitcherPanel ResetCamera))

(event `self.ReceiveTick`
  (params (DeltaSeconds :type "Float (single-precision)"))
  ;[0 0.8359 1] Tick
  (set `self.TimeSinceLastScroll` (+ (`self.TimeSinceLastScroll`) DeltaSeconds))
  (set `self.TimeSinceLeftMousePressed` (+ (`self.TimeSinceLeftMousePressed`) DeltaSeconds))
  (`/Engine/EditorBlueprintResources/StandardMacros.IsValid` (`self.MapCamera`)
    (:`Is Valid`
      (`self.Update Map Camera`))))

(event `InputAxis|LookVertical`
  (params (AxisValue :type "Float (single-precision)"))
  ;[1 0.9141 0] Input
  (if (`self.CanRotateCamera`)
    (`self.RotateVertically` AxisValue)))

(event `InputAction|MouseWheelUp`
  (params (Key :type "Key Structure"))
  ;[1 0.9141 0] Input
  (:`Pressed`
    (if (>= (`self.TimeSinceLastScroll`) (`self.DelayBetweenScrolling`))
      (`/Game/Kambio/Blueprints/UI/Component_UIConfig.MaybeScrollToLastSwitcherPanel` (`self.UIConfigComponent`))
      (set `self.TimeSinceLastScroll` 0.0 :!label _label))))

(event `InputAction|MouseWheelDown`
  (params (Key :type "Key Structure"))
  ;[1 0.9141 0] Input
  (:`Pressed`
    (if (>= (`self.TimeSinceLastScroll`) (`self.DelayBetweenScrolling`))
      (`/Game/Kambio/Blueprints/UI/Component_UIConfig.MaybeScrollToNextSwitcherPanel` (`self.UIConfigComponent`))
      (goto _label))))

(event `InputAction|SendScreenshot`
  (params (Key :type "Key Structure"))
  ;[1 0.9141 0] Input
  (:`Pressed`
    (bind (_texture2d _outpixelcolors _outbinaryimage) (`EasyScreenshot.TakeScreenshot` 1920 1080 false (`KismetStringLibrary.Concat_StrStr` (`KismetSystemLibrary.GetDisplayName` (`self.CurrentCamera`)) "_Screenshot") "")
      (:`OnSuccess`
        (`PixelStreamingBlueprints.SendFileAsByteArray` _outbinaryimage "image/png" "png")))))

(fn `GoToCinematicMode`
  (if (not (`|EnumEquality` (`self.CurrentAppMode`) "NewEnumerator2"))
    (set `self.CurrentAppMode` "NewEnumerator2")
    (`/Game/Kambio/Blueprints/UI/Component_UIConfig.InstantiateHUDSmall` (`self.UIConfigComponent`) "NewEnumerator2")
    (`/Game/Kambio/Blueprints/Gameplay/SequenceComponent.RunSequencer` (`self.SequenceComponent`))))

(fn `GoToConfigurationMode`
  (bind _currentcamera (`self.CurrentCamera`))
  (if (not (`|EnumEquality` (`self.CurrentAppMode`) "NewEnumerator0"))
    (set `/Game/Kambio/Blueprints/Gameplay/SequenceComponent.SequenceIsRunning` false (`self.SequenceComponent`))
    (`/Engine/EditorBlueprintResources/StandardMacros.IsValid` _currentcamera
      (:`Is Valid`
        (set `/Game/Kambio/Blueprints/Camera/BP_CustomCamera.IsExploring` false _currentcamera))
      (:`Is Not Valid`
        _))
    (set `self.CurrentAppMode` "NewEnumerator0")
    (`/Game/Kambio/Blueprints/UI/Component_UIConfig.InstantiateHUD` (`self.UIConfigComponent`))
    (set `self.CanActivateCameraRotation` true)))

(fn `GoToExplorationMode`
  (if (not (`|EnumEquality` (`self.CurrentAppMode`) "NewEnumerator1"))
    (set `/Game/Kambio/Blueprints/Gameplay/SequenceComponent.SequenceIsRunning` false (`self.SequenceComponent`))
    (bind _outactors (`GameplayStatics.GetAllActorsOfClassWithTag` "/Game/Kambio/Blueprints/Camera/BP_CustomCamera.BP_CustomCamera_C" (`KismetStringLibrary.Conv_StringToName` (`/Game/Kambio/DataAssets/Config/PDAs/PDA_ConfigGameplay.InitCameraTagForExploration` (`self.DA_ConfigGameplay`)))))
    (bind _output_get (set `self.CurrentCamera` (`|GetArrayItem` _outactors)))
    (set `/Game/Kambio/Blueprints/Camera/BP_CustomCamera.IsExploring` true _output_get)
    (`/Game/Kambio/Blueprints/Camera/BP_CustomCamera.ShowArrow` _output_get)
    (`self.Set New Camera` _output_get true true)
    (set `self.CanRotateCamera` true)
    (set `self.CurrentAppMode` "NewEnumerator1")
    (`/Game/Kambio/Blueprints/UI/Component_UIConfig.InstantiateHUDSmall` (`self.UIConfigComponent`) "NewEnumerator1")))

(fn `HideMeshesByCurrentCamera`
  (for _array_element (`/Game/Kambio/Blueprints/Camera/BP_CustomCamera.MeshesToHide` (`self.CurrentCamera`))
    (`SceneComponent.SetVisibility` (`StaticMeshActor.StaticMeshComponent` _array_element) false true)))

(fn `RotateHorizontally`
  (params (AxisValue :type "Float (double-precision)"))
  (bind _returnvalue (* AxisValue (`GameplayStatics.GetWorldDeltaSeconds`) (`self.RotationSpeed`) -1.0))
  ;[0.4766 1 0] Rotate current character horizontally and call event LookHorizontal
  (`Pawn.AddControllerYawInput` (`GameplayStatics.GetPlayerCharacter` 0) _returnvalue)
  (`self.EventLookHorizontal` _returnvalue))

(fn `RotateVertically`
  (params (AxisValue :type "Float (double-precision)"))
  (bind _returnvalue (* AxisValue (`GameplayStatics.GetWorldDeltaSeconds`) (`self.RotationSpeed`)))
  ;[0.9922 0 1] Rotate current character vertically and send event LookVertical
  (`Pawn.AddControllerPitchInput` (`GameplayStatics.GetPlayerCharacter` 0) _returnvalue)
  (`self.EventLookVertical` _returnvalue))

(fn `Set New Camera`
  (params (CustomCamera :type "/Game/Kambio/Blueprints/Camera/BP_CustomCamera Object Reference") (CanRotate :type Boolean) (ResetView :type Boolean) (BlendTime :type "Float (double-precision)" :default 1.0))
  (bind _currentcamera (`self.CurrentCamera`))
  ;[0 1 0.5078] Set Associated Camera as new View Target
  (set `/Game/Kambio/Blueprints/Camera/BP_CustomCamera.CanRotate` CanRotate CustomCamera)
  (`self.ShowMeshesByCurrentCamera`)
  (if (`KismetSystemLibrary.IsValid` _currentcamera)
    (set `/Game/Kambio/Blueprints/Camera/BP_CustomCamera.IsActive` false _currentcamera))
  (if ResetView
    (`/Game/Kambio/Blueprints/Camera/BP_CustomCamera.ReturnToInitialSetup` CustomCamera))
  (bind _output_get (set `self.CurrentCamera` CustomCamera))
  (`/Game/Kambio/Blueprints/Camera/BP_MapCamera.SetIgnoreMeshesByFloorTag` (`self.MapCamera`) (`/Game/Kambio/Blueprints/Camera/BP_CustomCamera.FloorId` _output_get))
  (set `/Game/Kambio/Blueprints/Camera/BP_CustomCamera.IsActive` true _output_get)
  (`self.SetViewTargetWithBlend` _output_get BlendTime)
  (`self.HideMeshesByCurrentCamera`))

(fn `SetNewCameraForConfiguration`
  (params (SwitcherPanel :type "/Game/Kambio/Blueprints/UI/Widgets/Panels/Widget_SwitcherPanel Object Reference") (`Reset Camera` :type Boolean))
  (bind _currentcamera (`self.CurrentCamera`))
  (bind _da_switcherpanel (`/Game/Kambio/Blueprints/UI/Widgets/Panels/Widget_SwitcherPanel.DA_SwitcherPanel` SwitcherPanel))
  ;[0 1 0.5078] Set Associated Camera as new View Target
  (`/Engine/EditorBlueprintResources/StandardMacros.IsValid` _currentcamera
    (:`Is Valid`
      (`/Game/Kambio/Blueprints/Camera/BP_CustomCamera.HideArrow` _currentcamera))
    (:`Is Not Valid`
      _))
  (bind _outactors (`GameplayStatics.GetAllActorsOfClassWithTag` "/Game/Kambio/Blueprints/Camera/BP_CustomCamera.BP_CustomCamera_C" (`KismetStringLibrary.Conv_StringToName` (`/Game/Kambio/DataAssets/Panels/PDA_SwitcherPanel.CameraTag` _da_switcherpanel))))
  (if (> (`KismetArrayLibrary.Array_Length` _outactors) 0)
    (bind _output (`|GetArrayItem` _outactors))
    (`/Engine/EditorBlueprintResources/StandardMacros.IsValid` _output
      (:`Is Valid`
        (`self.Set New Camera` _output (`/Game/Kambio/DataAssets/Panels/PDA_SwitcherPanel.CanRotateCamera` _da_switcherpanel) `Reset Camera`)))))

(fn `SetNewCameraForExploration`
  (bind _currentcamera (`self.CurrentCamera`))
  (bind _camerawithsmallestangle (`/Game/Kambio/Blueprints/Camera/BP_CustomCamera.CameraWithSmallestAngle` (`self.CurrentCamera`)))
  (set `/Game/Kambio/Blueprints/Camera/BP_CustomCamera.IsExploring` false _currentcamera)
  (`/Game/Kambio/Blueprints/Camera/BP_CustomCamera.HideArrow` _currentcamera)
  (`/Engine/EditorBlueprintResources/StandardMacros.IsValid` _camerawithsmallestangle
    (:`Is Valid`
      (set `/Game/Kambio/Blueprints/Camera/BP_CustomCamera.IsExploring` true _camerawithsmallestangle)
      (`/Game/Kambio/Blueprints/Camera/BP_CustomCamera.ShowArrow` _camerawithsmallestangle)
      (`self.Set New Camera` _camerawithsmallestangle true true))))

(fn `ShowMeshesByCurrentCamera`
  (if (`KismetSystemLibrary.IsValid` (`self.CurrentCamera`))
    (for _array_element (`/Game/Kambio/Blueprints/Camera/BP_CustomCamera.MeshesToHide` (`self.CurrentCamera`))
      (`SceneComponent.SetVisibility` (`StaticMeshActor.StaticMeshComponent` _array_element) true true))))

(fn `Update Map Camera`
  (bind _mapcamera (`self.MapCamera`))
  (`/Engine/EditorBlueprintResources/StandardMacros.IsValid` (`self.CurrentCamera`)
    (:`Is Valid`
      (`SceneComponent.K2_SetWorldLocation` (`SceneCapture.SceneComponent` (`self.MapCamera`)) (`KismetMathLibrary.MakeVector` (.x (`SceneComponent.K2_GetComponentLocation` (`CameraActor.SceneComponent` (`self.CurrentCamera`)))) (.y (`SceneComponent.K2_GetComponentLocation` (`CameraActor.SceneComponent` (`self.CurrentCamera`)))) (+ (.z (`SceneComponent.K2_GetComponentLocation` (`CameraActor.SceneComponent` (`self.CurrentCamera`)))) (`/Game/Kambio/DataAssets/Config/PDAs/PDA_ConfigGameplay.CameraMapZValue` (`self.DA_ConfigGameplay`)))) false false)
      (`SceneComponent.K2_SetWorldRotation` (`Actor.RootComponent` _mapcamera) (`KismetMathLibrary.FindLookAtRotation` (`SceneComponent.K2_GetComponentLocation` (`SceneCapture.SceneComponent` _mapcamera)) (`SceneComponent.K2_GetComponentLocation` (`CameraActor.SceneComponent` (`self.CurrentCamera`)))) false false))))

(fn `UserConstructionScript`)