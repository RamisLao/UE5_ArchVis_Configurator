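; Player controller for a material-switching viewer with a mouse-driven UI and player character navigation.
; On BeginPlay it builds a HUD selector panel with one button per MaterialManager material, each applying its material to slot 0 of the group's meshes.
; Axis inputs drive movement, plus camera rotation while middle mouse is held, with look deltas also broadcast as events.
; Keys 1 and 2 fire events and lock movement; E fires its own and unlocks it.
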(event `self.ReceiveBeginPlay`
  ;[1 1 1] Setup
  (`KismetSystemLibrary.Delay` 1.0)
  (set `self.bShowMouseCursor` true)
  (bind _returnvalue (`|CreateWidget` "/Game/Kambio/Blueprints/UI/Widget_HUD.Widget_HUD_C" self))
  (bind _output_get (set `self.WidgetHUD` _returnvalue))
  (`UserWidget.AddToViewport` _output_get 0)
  (bind _returnvalue_2 (`|CreateWidget` "/Game/Kambio/Blueprints/UI/Widget_SelectorPanel.Widget_SelectorPanel_C" self))
  (`PanelWidget.AddChild` (`/Game/Kambio/Blueprints/UI/Widget_HUD.WidgetSwitcher` (`self.WidgetHUD`)) _returnvalue_2)
  (for _array_element (`/Game/Kambio/Blueprints/BP_MatChangeGroup.Materials` (`/Game/Kambio/Blueprints/BP_MaterialManager.MatChangeGroup` (`self.MaterialManager`)))
    (bind _returnvalue_3 (`|CreateWidget` "/Game/Kambio/Blueprints/UI/Widget_MatButton.Widget_MatButton_C"))
    (set `/Game/Kambio/Blueprints/UI/Widget_MatButton.Material` _array_element _returnvalue_3)
    (add `/Game/Kambio/Blueprints/UI/Widget_MatButton.ButtonClicked` _returnvalue_3 (delegate `CustomEvent_0`))
    (`PanelWidget.AddChild` (`/Game/Kambio/Blueprints/UI/Widget_SelectorPanel.HorizontalBox` _returnvalue_2) _returnvalue_3)))

(event `CustomEvent_0`
  (params (Material :type "MaterialInstance Object Reference"))
  (for _array_element (`/Game/Kambio/Blueprints/BP_MatChangeGroup.Meshes` (`/Game/Kambio/Blueprints/BP_MaterialManager.MatChangeGroup` (`self.MaterialManager`)))
    (`PrimitiveComponent.SetMaterial` (`StaticMeshActor.StaticMeshComponent` _array_element) 0 Material)))

(event `InputAxis|MoveForward`
  (params (AxisValue :type "Float (single-precision)"))
  ;[1 1 1] Movement
  (if (`self.CanMoveFreely`)
    (`Pawn.AddMovementInput` (`GameplayStatics.GetPlayerCharacter` 0) (`self.GetActorForwardVector`) (* AxisValue (`GameplayStatics.GetWorldDeltaSeconds`) (`self.MovementSpeed`)) false)))

(event `InputAxis|MoveRight`
  (params (AxisValue :type "Float (single-precision)"))
  ;[1 1 1] Movement
  (if (`self.CanMoveFreely`)
    (`Pawn.AddMovementInput` (`GameplayStatics.GetPlayerCharacter` 0) (`self.GetActorRightVector`) (* AxisValue (`GameplayStatics.GetWorldDeltaSeconds`) (`self.MovementSpeed`)) false)))

(event `InputAxis|LookHorizontal`
  (params (AxisValue :type "Float (single-precision)"))
  (bind _returnvalue (* AxisValue (`GameplayStatics.GetWorldDeltaSeconds`) (`self.RotationSpeed`)))
  ;[1 1 1] Camera Rotation
  (if (`self.CanRotateCamera`)
    (`Pawn.AddControllerYawInput` (`GameplayStatics.GetPlayerCharacter` 0) _returnvalue)
    (`self.EventLookHorizontal` _returnvalue)))

(event `Key|MiddleMouseButton`
  (params (Key :type "Key Structure"))
  ;[1 1 1] Camera Rotation
  (:`Pressed`
    (set `self.CanRotateCamera` true))
  (:`Released`
    (set `self.CanRotateCamera` false)))

(event `InputAxis|LookVertical`
  (params (AxisValue :type "Float (single-precision)"))
  (bind _returnvalue (* AxisValue -1.0 (`GameplayStatics.GetWorldDeltaSeconds`) (`self.RotationSpeed`)))
  ;[1 1 1] Camera Rotation
  (if (`self.CanRotateCamera`)
    (`Pawn.AddControllerPitchInput` (`GameplayStatics.GetPlayerCharacter` 0) _returnvalue)
    (`self.EventLookVertical` _returnvalue)))

(event `Key|One`
  (params (Key :type "Key Structure"))
  (:`Pressed`
    (`self.EventPressed1`)
    (set `self.CanMoveFreely` false)))

(event `Key|Two`
  (params (Key :type "Key Structure"))
  (:`Pressed`
    (`self.EventPressed2`)
    (set `self.CanMoveFreely` false)))

(event `Key|E`
  (params (Key :type "Key Structure"))
  (:`Pressed`
    (`self.EventPressedE`)
    (set `self.CanMoveFreely` true)))

(fn `UserConstructionScript`)