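; BP_StaticCamera is a camera Blueprint that rotates its camera component from player look input.
; On BeginPlay it casts the first player controller to BP_KambioPlayerController and binds to its horizontal and vertical look events.
; Horizontal values add relative yaw and negated vertical values add relative pitch, with no clamping or frame-time scaling in this Blueprint.
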(event `self.ReceiveBeginPlay`
  (bind _asbp_kambio_player_controller (cast `/Game/Kambio/Blueprints/BP_KambioPlayerController` (`GameplayStatics.GetPlayerController` 0)))
  (add `/Game/Kambio/Blueprints/BP_KambioPlayerController.EventLookHorizontal` _asbp_kambio_player_controller (delegate `OnLookHorizontal`))
  (add `/Game/Kambio/Blueprints/BP_KambioPlayerController.EventLookVertical` _asbp_kambio_player_controller (delegate `CustomEvent_0`)))

(event `OnLookHorizontal`
  (params (Value :type "Float (double-precision)"))
  (`SceneComponent.K2_AddRelativeRotation` (`self.CameraComponent`) (`KismetMathLibrary.MakeRotator` 0.0 0.0 Value) false false))

(event `CustomEvent_0`
  (params (Value :type "Float (double-precision)"))
  (`SceneComponent.K2_AddRelativeRotation` (`self.CameraComponent`) (`KismetMathLibrary.MakeRotator` 0.0 (* Value -1.0)) false false))

(fn `UserConstructionScript`)