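; Configurator component that applies design options, stored as option-to-value pairs in DAConfig, to tagged scene meshes.
; UpdateOptionId uses data-asset lookups to route each option to a material swap or visibility toggle, then records the value.
; Material changes cascade to influenced options still matching the influencer's previous material.
; Button handlers feed these updates; other functions show or hide floors by model variation and send the config as JSON over Pixel Streaming.
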(fn `ApplyAllConfigs`
  (bind _optionidtovalue (`/Game/Kambio/DataAssets/Config/PDAs/PDA_Config.OptionIdToValue` (`self.DA_Config`)))
  ;[1 0 0.4219] Iterate through all TagToConfig and apply the configuration to the static meshes
  (bind _keys (`BlueprintMapLibrary.Map_Keys` _optionidtovalue))
  (for _array_element _keys
    (`self.UpdateOptionId` _array_element (`BlueprintMapLibrary.Map_Find` _optionidtovalue _array_element))))

(fn `ButtonMaterialIdClicked`
  (params (DAButton :type "/Game/Kambio/DataAssets/Buttons/PDA_ItemMaterialId Object Reference") (OwningDAScrollPanel :type "/Game/Kambio/DataAssets/Panels/PDA_ScrollPanel Object Reference"))
  ;[0.6641 1 0] Update Tag Material using General Tag and selected Material
  (for _array_element (`/Game/Kambio/DataAssets/Panels/PDA_ScrollPanel.Tags` OwningDAScrollPanel)
    (`self.UpdateOptionIdMaterial` _array_element (`/Game/Kambio/DataAssets/Buttons/PDA_ItemMaterialId.MaterialId` DAButton))))

(fn `ButtonOptionIdToMaterialIdClicked`
  (params (DAButton :type "/Game/Kambio/DataAssets/Buttons/PDA_ItemOptionIdToMaterialId Object Reference") (OwningDAScrollPanel :type "/Game/Kambio/DataAssets/Panels/PDA_ScrollPanel Object Reference"))
  (bind _optionidtomaterialid (`/Game/Kambio/DataAssets/Buttons/PDA_ItemOptionIdToMaterialId.OptionIdToMaterialId` DAButton))
  ;[1 0 0.9844] Iterate through all TagToMaterial keys and call Update Tag Material with each one
  (bind _keys (`BlueprintMapLibrary.Map_Keys` _optionidtomaterialid))
  (for _array_element _keys
    (`self.UpdateOptionIdMaterial` _array_element (`BlueprintMapLibrary.Map_Find` _optionidtomaterialid _array_element))))

(fn `ButtonOptionIdToOptionIdClicked`
  (params (DAButton :type "/Game/Kambio/DataAssets/Buttons/PDA_ItemOptionIdToOptionId Object Reference") (OwningDAScrollPanel :type "/Game/Kambio/DataAssets/Panels/PDA_ScrollPanel Object Reference"))
  (bind _optionidtooptionid (`/Game/Kambio/DataAssets/Buttons/PDA_ItemOptionIdToOptionId.OptionIdToOptionId` DAButton))
  (bind _optionidtovalue (`/Game/Kambio/DataAssets/Config/PDAs/PDA_Config.OptionIdToValue` (`self.DA_Config`)))
  (bind _keys (`BlueprintMapLibrary.Map_Keys` _optionidtooptionid))
  (for _array_element _keys
    (bind _value (`BlueprintMapLibrary.Map_Find` _optionidtooptionid _array_element))
    (if (`BlueprintMapLibrary.Map_Contains` _optionidtovalue _value)
      (`self.UpdateOptionId` _array_element (`BlueprintMapLibrary.Map_Find` _optionidtovalue _value))
      (else
        (`KismetSystemLibrary.PrintString` (`KismetStringLibrary.Concat_StrStr` "ButtonOptionIdToOptionId - Error! " "The following Tag: " "\"" _array_element "\"" " references a Tag that was not found in DA Config: " "\"" _value "\"") true true (struct :`G` 0.66 :`B` 1.0 :`A` 1.0) 10.0)))))

(fn `ButtonOptionIdToSelectionIdClicked`
  (params (DAButton :type "/Game/Kambio/DataAssets/Buttons/PDA_ItemOptionIdToSelectionId Object Reference") (OwningDAScrollPanel :type "/Game/Kambio/DataAssets/Panels/PDA_ScrollPanel Object Reference"))
  (bind _optionidtoselectionid (`/Game/Kambio/DataAssets/Buttons/PDA_ItemOptionIdToSelectionId.OptionIdToSelectionId` DAButton))
  (bind _keys (`BlueprintMapLibrary.Map_Keys` _optionidtoselectionid))
  (for _array_element _keys
    (`self.UpdateOptionIdSelection` _array_element (`BlueprintMapLibrary.Map_Find` _optionidtoselectionid _array_element))))

(fn `CleanDAConfig`
  (locals (CurrentValue :type String))
  (bind _optionidtovalue (`/Game/Kambio/DataAssets/Config/PDAs/PDA_Config.OptionIdToValue` (`self.DA_Config`)))
  ;[0.03125 1 0] Remove all spaces from tags, to avoid having repeated tags with small differences
  (bind _keys (`BlueprintMapLibrary.Map_Keys` _optionidtovalue))
  (for _array_element _keys
    (set `local.CurrentValue` (`BlueprintMapLibrary.Map_Find` _optionidtovalue _array_element))
    (`BlueprintMapLibrary.Map_Remove` _optionidtovalue _array_element)
    (`BlueprintMapLibrary.Map_Add` _optionidtovalue (`KismetStringLibrary.Replace` _array_element " ") (`local.CurrentValue`))))

(fn `HideShowMeshesAccordingToVariation`
  (for _array_element (`/Game/Kambio/DataAssets/Config/PDAs/PDA_ConfigFloors.VariationIdsToFloorsIds` (`self.DA_ConfigVariations`))
    (if (`KismetStringLibrary.EqualEqual_StrStr` (`/Game/Kambio/DataAssets/Config/PDAs/PDA_VariationIdToFloorIds.VariationId` _array_element) (`/Game/Kambio/DataAssets/Config/PDAs/PDA_ModelAndVariation.VariationId` (`self.DA_ModelAndVariation`)))
      (for _array_element_2 (`/Game/Kambio/DataAssets/Config/PDAs/PDA_VariationIdToFloorIds.FloorIdsToShow` _array_element)
        (bind _outactors (`GameplayStatics.GetAllActorsWithTag` (`KismetStringLibrary.Conv_StringToName` _array_element_2)))
        (for _array_element_3 _outactors
          (`Actor.SetActorHiddenInGame` _array_element_3 false)))
      (for _array_element_4 (`/Game/Kambio/DataAssets/Config/PDAs/PDA_VariationIdToFloorIds.FloorIdsToHide` _array_element)
        (bind _outactors_2 (`GameplayStatics.GetAllActorsWithTag` (`KismetStringLibrary.Conv_StringToName` _array_element_4)))
        (for _array_element_5 _outactors_2
          (`Actor.SetActorHiddenInGame` _array_element_5 true)))
      (break))))

(fn `MaybeOptionIdInfluencesOtherOptionId`
  (params (Tag :type String) (NewMaterialName :type String))
  (bind (_value _returnvalue) (`BlueprintMapLibrary.Map_Find` (`/Game/Kambio/DataAssets/Config/PDAs/PDA_Config.OptionIdToValue` (`self.DA_Config`)) Tag))
  ;[0 1 0.1094] Check if Tag is an Influencer of other Tags. If it is, check if the Influenced Tag has the same Material as the Influencer. If it does, change the Influenced Tag to the new Material
  (for _array_element (`/Game/Kambio/DataAssets/Config/PDAs/PDA_ActiveInfluences.Influences` (`self.DA_ActiveInfluences`))
    (if (`KismetStringLibrary.EqualEqual_StrStr` Tag (`KismetStringLibrary.Replace` (`/Game/Kambio/DataAssets/Config/PDAs/PDA_Influence.InfluencerTag` _array_element) " "))
      (if _returnvalue
        (for _array_element_2 (`/Game/Kambio/DataAssets/Config/PDAs/PDA_Influence.InfluencedTags` _array_element)
          (bind _returnvalue_2 (`KismetStringLibrary.Replace` _array_element_2 " "))
          (bind (_value_2 _returnvalue_3) (`BlueprintMapLibrary.Map_Find` (`/Game/Kambio/DataAssets/Config/PDAs/PDA_Config.OptionIdToValue` (`self.DA_Config`)) _returnvalue_2))
          (if _returnvalue_3
            (if (`KismetStringLibrary.EqualEqual_StrStr` _value_2 _value)
              (`self.UpdateOptionId` _returnvalue_2 NewMaterialName) ; If it is the same, then change the Influenced Tag to the new Parameter
            )))
        (break)))))

(fn `SendDataByPixelStreamingResponse`
  (locals (DesignOptions :type "Array of JsonObjectWrapper Structure") (JsonData :type "JsonObjectWrapper Structure"))
  (bind _outjsonobject (`JsonBlueprintFunctionLibrary.FromString` "{}"))
  (set `local.JsonData` _outjsonobject)
  (bind _keys (`BlueprintMapLibrary.Map_Keys` (`/Game/Kambio/DataAssets/Config/PDAs/PDA_Config.OptionIdToValue` (`self.DA_Config`))))
  (for _array_element _keys
    (bind _outjsonobject_2 (`JsonBlueprintFunctionLibrary.FromString` "{}"))
    (`|SetJsonField` _outjsonobject_2 "optionId" _array_element)
    (`|SetJsonField` _outjsonobject_2 "valueId" (`BlueprintMapLibrary.Map_Find` (`/Game/Kambio/DataAssets/Config/PDAs/PDA_Config.OptionIdToValue` (`self.DA_Config`)) _array_element))
    (`KismetArrayLibrary.Array_Add` (`local.DesignOptions`) _outjsonobject_2))
  (`|SetJsonField` (`local.JsonData`) "designOptions" (`local.DesignOptions`))
  (bind _outjsonstring (`JsonBlueprintFunctionLibrary.ToString` (`local.JsonData`)))
  (`KismetSystemLibrary.PrintString` _outjsonstring)
  (bind _asbp_kambio_player_controller (cast `/Game/Kambio/Blueprints/Gameplay/BP_KambioPlayerController` (`GameplayStatics.GetPlayerController` 0)))
  (`PixelStreamingInput.SendPixelStreamingResponse` (`/Game/Kambio/Blueprints/Gameplay/BP_KambioPlayerController.PixelStreamingInput` _asbp_kambio_player_controller) _outjsonstring))

(fn `UpdateOptionId`
  (params (OptionId :type String) (Value :type String))
  (locals (L_IdToUpdate :type String) (L_Value :type String))
  ;[1 0 0.7031] Receive a Tag and an UpdateParam and call the appropriate function to update all objects with Tag
  (set `local.L_Value` Value)
  (set `local.L_IdToUpdate` OptionId)
  (if (`BlueprintMapLibrary.Map_Contains` (`/Game/Kambio/DataAssets/Config/PDAs/PDA_Config.OptionIdToValue` (`self.DA_Config`)) (`local.L_IdToUpdate`))
    (if (`|EnumEquality` (`BlueprintMapLibrary.Map_Find` (`/Game/Kambio/DataAssets/Config/PDAs/PDA_OptionIdToOptionType.OptionIdToOptionType` (`self.DA_OptionIdToOptionType`)) (`local.L_IdToUpdate`)) "NewEnumerator0")
      (`self.UpdateOptionIdMaterial` (`local.L_IdToUpdate`) (`local.L_Value`))
      (elif (`|EnumEquality` (`BlueprintMapLibrary.Map_Find` (`/Game/Kambio/DataAssets/Config/PDAs/PDA_OptionIdToOptionType.OptionIdToOptionType` (`self.DA_OptionIdToOptionType`)) (`local.L_IdToUpdate`)) "NewEnumerator1")
        (`self.UpdateOptionIdSelection` (`local.L_IdToUpdate`) (`local.L_Value`))
        (else
          (`KismetSystemLibrary.PrintString` (`KismetStringLibrary.Concat_StrStr` "Error! " "Update of Tag \"" (`local.L_IdToUpdate`) "\" failed. The following UpdateParam has a syntax error: " (`local.L_Value`)) true true (struct :`G` 0.66 :`B` 1.0 :`A` 1.0) 10.0))))
    (else
      (`KismetSystemLibrary.PrintString` (`KismetStringLibrary.Concat_StrStr` "UpdateOptionId - Error! " "The following tag was not found in the DA_Config file: " (`local.L_IdToUpdate`)) true true (struct :`G` 0.66 :`B` 1.0 :`A` 1.0) 10.0))))

(fn `UpdateOptionIdMaterial`
  (params (OptionId :type String) (MaterialId :type String))
  (bind _returnvalue (`KismetStringLibrary.Replace` OptionId " "))
  (bind (_value _returnvalue_2) (`BlueprintMapLibrary.Map_Find` (`/Game/Kambio/DataAssets/Config/PDAs/PDA_MaterialIdToMaterialInstance.MaterialIdToMaterialInstance` (`self.DA_MaterialIdToMaterialInstance`)) MaterialId))
  ;[0 1 0.1562] Apply Material to all StaticMeshes with Tag
  (if _returnvalue_2
    (`self.MaybeOptionIdInfluencesOtherOptionId` OptionId MaterialId)
    (bind _outactors (`GameplayStatics.GetAllActorsOfClassWithTag` "/Script/Engine.StaticMeshActor" (`KismetStringLibrary.Conv_StringToName` _returnvalue)))
    (for _array_element _outactors
      (`PrimitiveComponent.SetMaterial` (`StaticMeshActor.StaticMeshComponent` _array_element) 0 _value))
    (`BlueprintMapLibrary.Map_Add` (`/Game/Kambio/DataAssets/Config/PDAs/PDA_Config.OptionIdToValue` (`self.DA_Config`)) _returnvalue MaterialId)
    (else
      (`KismetSystemLibrary.PrintString` (`KismetStringLibrary.Concat_StrStr` "Error! " "The following material was not found in the Materials database: " MaterialId " / OptionId: " OptionId) true true (struct :`G` 0.66 :`B` 1.0 :`A` 1.0) 10.0))))

(fn `UpdateOptionIdSelection`
  (params (OptionId :type String) (SelectionId :type String))
  (bind _value (`BlueprintMapLibrary.Map_Find` (`/Game/Kambio/DataAssets/Config/PDAs/PDA_SelectionIdToVisibility.SelectionIdToVisibility` (`self.DA_SelectionIdToVisibility`)) SelectionId))
  ;[1 0.9609 0] Update Static Meshes with Tag to be visible or not according to Selection
  (bind _outactors (`GameplayStatics.GetAllActorsOfClassWithTag` "/Script/Engine.StaticMeshActor" (`KismetStringLibrary.Conv_StringToName` OptionId)))
  (if (== _value true)
    (for _array_element _outactors
      (`SceneComponent.SetVisibility` (`Actor.RootComponent` _array_element) true true))
    (`BlueprintMapLibrary.Map_Add` (`/Game/Kambio/DataAssets/Config/PDAs/PDA_Config.OptionIdToValue` (`self.DA_Config`)) OptionId SelectionId :!label _label)
    (elif (== _value false)
      (for _array_element_2 _outactors
        (`SceneComponent.SetVisibility` (`Actor.RootComponent` _array_element_2) false true))
      (goto _label)
      (else
        (`KismetSystemLibrary.PrintString` (`KismetStringLibrary.Concat_StrStr` "Error! " "The following Visibility Tag is not valid: " SelectionId) true true (struct :`G` 0.66 :`B` 1.0 :`A` 1.0) 10.0)))))