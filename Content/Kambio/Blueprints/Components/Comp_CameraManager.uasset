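; Player controller component that manages the active BP_CustomCamera and the overhead map camera, and sends PNG screenshots on input.
; SetNewCamera blends the view target, swaps each camera's hidden meshes and view plane, and updates the map's floor filter.
; Configuration picks cameras by switcher-panel tag; exploration moves to CameraWithSmallestAngle, aimed at the current line of sight.
; Tick keeps the map camera above the current camera, looking down at it.
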(event `self.ReceiveTick`
  (params (DeltaSeconds :type "Float (single-precision)"))
  (`/Engine/EditorBlueprintResources/StandardMacros.IsValid` (`self.MapCamera`)
    (:`Is Valid`
      (`self.Update Map Camera`))))

(event `InputAction|SendScreenshot`
  (params (Key :type "Key Structure"))
  (:`Pressed`
    (bind (_texture2d _outpixelcolors _outbinaryimage) (`EasyScreenshot.TakeScreenshot` 1920 1080 false (`KismetStringLibrary.Concat_StrStr` (`KismetSystemLibrary.GetDisplayName` (`self.CurrentCamera`)) "_Screenshot") "")
      (:`OnSuccess`
        (`PixelStreamingBlueprints.SendFileAsByteArray` _outbinaryimage "image/png" "png")))))

(fn `HideMeshesByCurrentCamera`
  (for _array_element (`/Game/Kambio/Blueprints/Cameras/BP_CustomCamera.MeshesToHide` (`self.CurrentCamera`))
    (`SceneComponent.SetVisibility` (`StaticMeshActor.StaticMeshComponent` _array_element) false true)))

(fn `Set New Camera`
  (params (CustomCamera :type "/Game/Kambio/Blueprints/Cameras/BP_CustomCamera Object Reference") (CanRotate :type Boolean) (ResetView :type Boolean) (BlendTime :type "Float (double-precision)" :default 1.0))
  (bind _currentcamera (`self.CurrentCamera`))
  ;[0 1 0.5078] Set Associated Camera as new View Target
  (set `/Game/Kambio/Blueprints/Cameras/BP_CustomCamera.CanRotate` CanRotate CustomCamera)
  (`self.ShowMeshesByCurrentCamera`)
  (if (`KismetSystemLibrary.IsValid` _currentcamera)
    (`/Game/Kambio/Blueprints/Cameras/BP_CustomCamera.HideViewPlane` _currentcamera)
    (set `/Game/Kambio/Blueprints/Cameras/BP_CustomCamera.IsActive` false _currentcamera))
  (if ResetView
    (`/Game/Kambio/Blueprints/Cameras/BP_CustomCamera.ReturnToInitialSetup` CustomCamera))
  (bind _output_get (set `self.CurrentCamera` CustomCamera))
  (`/Game/Kambio/Blueprints/Cameras/BP_MapCamera.SetIgnoreMeshesByFloorTag` (`self.MapCamera`) (`/Game/Kambio/Blueprints/Cameras/BP_CustomCamera.SectionId` _output_get))
  (set `/Game/Kambio/Blueprints/Cameras/BP_CustomCamera.IsActive` true _output_get)
  (`/Game/Kambio/Blueprints/Cameras/BP_CustomCamera.ShowViewPlane` _output_get)
  (`PlayerController.SetViewTargetWithBlend` (`GameplayStatics.GetPlayerController` 0) _output_get BlendTime "VTBlend_Linear" 0.0 false)
  (`self.HideMeshesByCurrentCamera`))

(fn `SetNewCameraForConfiguration`
  (params (SwitcherPanel :type "/Game/Kambio/Blueprints/UI/Widgets/Panels/Widget_SwitcherPanel Object Reference") (`Reset Camera` :type Boolean))
  (bind _currentcamera (`self.CurrentCamera`))
  (bind _da_switcherpanel (`/Game/Kambio/Blueprints/UI/Widgets/Panels/Widget_SwitcherPanel.DA_SwitcherPanel` SwitcherPanel))
  ;[0 1 0.5078] Set Associated Camera as new View Target
  (`/Engine/EditorBlueprintResources/StandardMacros.IsValid` _currentcamera
    (:`Is Valid`
      (`/Game/Kambio/Blueprints/Cameras/BP_CustomCamera.HideArrow` _currentcamera))
    (:`Is Not Valid`
      _))
  (bind _outactors (`GameplayStatics.GetAllActorsOfClassWithTag` "/Game/Kambio/Blueprints/Cameras/BP_CustomCamera.BP_CustomCamera_C" (`KismetStringLibrary.Conv_StringToName` (`/Game/Kambio/DataAssets/PDAs/PDA_SwitcherPanel.CameraTag` _da_switcherpanel))))
  (if (> (`KismetArrayLibrary.Array_Length` _outactors) 0)
    (bind _output (`|GetArrayItem` _outactors))
    (`/Engine/EditorBlueprintResources/StandardMacros.IsValid` _output
      (:`Is Valid`
        (`self.Set New Camera` _output (`/Game/Kambio/DataAssets/PDAs/PDA_SwitcherPanel.CanRotateCamera` _da_switcherpanel) `Reset Camera`)))))

(fn `SetNewCameraForExploration`
  (locals (NewLookForward :type "Vector Structure"))
  (bind _currentcamera (`self.CurrentCamera`))
  (bind _cameracomponent (`CameraActor.CameraComponent` _currentcamera))
  (bind _camerawithsmallestangle (`/Game/Kambio/Blueprints/Cameras/BP_CustomCamera.CameraWithSmallestAngle` (`self.CurrentCamera`)))
  (bind _cameracomponent_2 (`CameraActor.CameraComponent` _camerawithsmallestangle))
  (set `/Game/Kambio/Blueprints/Cameras/BP_CustomCamera.IsExploring` false _currentcamera)
  (set `local.NewLookForward` (+ (`SceneComponent.K2_GetComponentLocation` _cameracomponent) (* (`SceneComponent.GetForwardVector` _cameracomponent) 100000.0)))
  (`/Game/Kambio/Blueprints/Cameras/BP_CustomCamera.HideArrow` _currentcamera)
  (`/Engine/EditorBlueprintResources/StandardMacros.IsValid` _camerawithsmallestangle
    (:`Is Valid`
      (set `/Game/Kambio/Blueprints/Cameras/BP_CustomCamera.IsExploring` true _camerawithsmallestangle)
      (`/Game/Kambio/Blueprints/Cameras/BP_CustomCamera.ShowArrow` _camerawithsmallestangle)
      (`SceneComponent.K2_SetWorldRotation` _cameracomponent_2 (`KismetMathLibrary.FindLookAtRotation` (`SceneComponent.K2_GetComponentLocation` _cameracomponent_2) (`local.NewLookForward`)) false false)
      (`self.Set New Camera` _camerawithsmallestangle true))))

(fn `ShowMeshesByCurrentCamera`
  (if (`KismetSystemLibrary.IsValid` (`self.CurrentCamera`))
    (for _array_element (`/Game/Kambio/Blueprints/Cameras/BP_CustomCamera.MeshesToHide` (`self.CurrentCamera`))
      (`SceneComponent.SetVisibility` (`StaticMeshActor.StaticMeshComponent` _array_element) true true))))

(fn `Update Map Camera`
  (bind _mapcamera (`self.MapCamera`))
  (`/Engine/EditorBlueprintResources/StandardMacros.IsValid` (`self.CurrentCamera`)
    (:`Is Valid`
      (bind _asbp_kambio_player_controller (cast `/Game/Kambio/Blueprints/Gameplay/BP_KambioPlayerController` (`self.GetOwner`)))
      (`SceneComponent.K2_SetWorldLocation` (`SceneCapture.SceneComponent` (`self.MapCamera`)) (`KismetMathLibrary.MakeVector` (.x (`SceneComponent.K2_GetComponentLocation` (`CameraActor.SceneComponent` (`self.CurrentCamera`)))) (.y (`SceneComponent.K2_GetComponentLocation` (`CameraActor.SceneComponent` (`self.CurrentCamera`)))) (+ (.z (`SceneComponent.K2_GetComponentLocation` (`CameraActor.SceneComponent` (`self.CurrentCamera`)))) (`/Game/Kambio/DataAssets/PDAs/PDA_ConfigGameplay.CameraMapZValue` (`/Game/Kambio/Blueprints/Gameplay/BP_KambioPlayerController.DA_ConfigGameplay` _asbp_kambio_player_controller)))) false false)
      (`SceneComponent.K2_SetWorldRotation` (`Actor.RootComponent` _mapcamera) (`KismetMathLibrary.FindLookAtRotation` (`SceneComponent.K2_GetComponentLocation` (`SceneCapture.SceneComponent` _mapcamera)) (`SceneComponent.K2_GetComponentLocation` (`CameraActor.SceneComponent` (`self.CurrentCamera`)))) false false))))