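; BP_KambioCharacter is a character Blueprint that handles movement and camera-look input.
; MoveForward and MoveRight share one chain, gated by CanMoveFreely, that applies movement along both the actor's forward and right vectors.
; Look axes drive controller yaw and inverted pitch.
; BeginPlay stores Camera as DefaultCamera, while a view-target blend to itself sits unconnected and never runs.
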(event `InputAxis|MoveForward`
  (params (AxisValue :type "Float (single-precision)"))
  ;[1 1 1] Movement
  (if (`self.CanMoveFreely`) :!label _label
    (`self.AddMovementInput` (`self.GetActorForwardVector`) AxisValue)
    (`self.AddMovementInput` (`self.GetActorRightVector`) (stale `InputAxis|MoveRight` AxisValue))))

(event `InputAxis|MoveRight`
  (params (AxisValue :type "Float (single-precision)"))
  ;[1 1 1] Movement
  (goto _label))

(event `InputAxis|LookHorizontal`
  (params (AxisValue :type "Float (single-precision)"))
  ;[1 1 1] Camera Rotation
  (`self.AddControllerYawInput` AxisValue))

(event `InputAxis|LookVertical`
  (params (AxisValue :type "Float (single-precision)"))
  ;[1 1 1] Camera Rotation
  (`self.AddControllerPitchInput` (* AxisValue -1.0)))

(event `self.ReceiveBeginPlay`
  (set `self.DefaultCamera` (`self.Camera`)))

(fn `UserConstructionScript`)