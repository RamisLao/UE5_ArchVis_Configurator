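; BP_Config is a configurator Blueprint that changes the material or visibility of tagged static mesh actors.
; UpdateTag validates tags against DAConfig, then routes by "Material" or "Visibility" in the tag name, printing errors for invalid input.
; Material names resolve through an enum to assets in DAIdToMaterial and are applied to slot 0.
; The TagToMaterial button handler applies each mapping directly; the other button handlers are empty.
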(event `self.ReceiveBeginPlay`
  (`parent.ReceiveBeginPlay`))

(fn `ButtonMaterialClicked`
  (params (DAButton :type "/Game/Kambio/Blueprints/DataAssets/Buttons/PDA_ButtonMaterial Object Reference") (OwningDAScrollPanel :type "/Game/Kambio/Blueprints/DataAssets/Panels/PDA_ScrollPanel Object Reference")))

(fn `ButtonTagToBooleanClicked`
  (params (DAButton :type "/Game/Kambio/Blueprints/DataAssets/Buttons/PDA_ButtonTagToBoolean Object Reference") (OwningDAScrollPanel :type "/Game/Kambio/Blueprints/DataAssets/Panels/PDA_ScrollPanel Object Reference")))

(fn `ButtonTagToMaterialClicked`
  (params (DAButton :type "/Game/Kambio/Blueprints/DataAssets/Buttons/PDA_ButtonTagToMaterial Object Reference") (OwningDAScrollPanel :type "/Game/Kambio/Blueprints/DataAssets/Panels/PDA_ScrollPanel Object Reference"))
  (bind _tagtomaterial (`/Game/Kambio/Blueprints/DataAssets/Buttons/PDA_ButtonTagToMaterial.TagToMaterial` DAButton))
  ;[0 1 0.5781] Iterate through all TagToMaterial keys and call Update Tag Material with each one
  (bind _keys (`BlueprintMapLibrary.Map_Keys` _tagtomaterial))
  (for _array_element _keys
    (`self.UpdateTagMaterial` _array_element (`BlueprintMapLibrary.Map_Find` _tagtomaterial _array_element))))

(fn `ButtonTagToTagClicked`
  (params (DAButton :type "/Game/Kambio/Blueprints/DataAssets/Buttons/PDA_ButtonTagToTag Object Reference") (OwningDAScrollPanel :type "/Game/Kambio/Blueprints/DataAssets/Panels/PDA_ScrollPanel Object Reference")))

(fn `GetEnumMaterialFromString`
  (params (String :type String))
  (returns (NewParam :type "/Game/Kambio/Blueprints/DataAssets/Config/Enum_Materials Enum"))
  ;[0 0.25 1] Receive a string with a Material name and get the corresponding Enum_Materials value
  (bind _enumvalue (foreach `/Game/Kambio/Blueprints/DataAssets/Config/Enum_Materials` false)
    (:`LoopBody`
      (if (`KismetStringLibrary.EqualEqual_StrStr` String (`|GetEnumeratorNameAsString` _enumvalue))
        (return _enumvalue)))))

(fn `UpdateTag`
  (params (Tag :type String) (UpdateParam :type String))
  (locals (L_TagToUpdate :type String) (L_UpdateParam :type String))
  ;[1 0 0.7031] Receive a Tag and an UpdateParam and call the appropriate function to update all objects with Tag
  (set `local.L_UpdateParam` UpdateParam)
  (set `local.L_TagToUpdate` Tag)
  (if (`BlueprintMapLibrary.Map_Contains` (`/Game/Kambio/Blueprints/DataAssets/Config/PDA_Config.TagToConfig` (`self.DAConfig`)) (`local.L_TagToUpdate`))
    (if (`KismetStringLibrary.Contains` (`local.L_TagToUpdate`) "Material")
      (bind _newparam (`self.GetEnumMaterialFromString` (`local.L_UpdateParam`)))
      (`self.UpdateTagMaterial` (`local.L_TagToUpdate`) _newparam)
      (elif (`KismetStringLibrary.Contains` (`local.L_TagToUpdate`) "Visibility")
        (`self.UpdateTagVisibility` (`local.L_TagToUpdate`) (`local.L_UpdateParam`))
        (else
          (`KismetSystemLibrary.PrintString` (`KismetStringLibrary.Concat_StrStr` "Error! " "Update of Tag \"" (`local.L_TagToUpdate`) "\" failed. The following UpdateParam has a syntax error: " (`local.L_UpdateParam`)) true true (struct :`G` 0.66 :`B` 1.0 :`A` 1.0) 10.0))))
    (else
      (`KismetSystemLibrary.PrintString` (`KismetStringLibrary.Concat_StrStr` "Error! " "The following tag was not found in the DA_Config file: " (`local.L_TagToUpdate`)) true true (struct :`G` 0.66 :`B` 1.0 :`A` 1.0) 10.0))))

(fn `UpdateTagMaterial`
  (params (Tag :type String) (Material :type "/Game/Kambio/Blueprints/DataAssets/Config/Enum_Materials Enum" :default "NewEnumerator0"))
  (bind (_value _returnvalue) (`BlueprintMapLibrary.Map_Find` (`/Game/Kambio/Blueprints/DataAssets/Config/PDA_IdToMaterial.IdToMaterial` (`self.DAIdToMaterial`)) Material))
  ;[0 1 0.1562] Apply Material to all StaticMeshes with Tag
  (if _returnvalue
    (bind _outactors (`GameplayStatics.GetAllActorsOfClassWithTag` "/Script/Engine.StaticMeshActor" (`KismetStringLibrary.Conv_StringToName` (`KismetStringLibrary.Replace` Tag " "))))
    (for _array_element _outactors
      (`PrimitiveComponent.SetMaterial` (`StaticMeshActor.StaticMeshComponent` _array_element) 0 _value))
    (else
      (`KismetSystemLibrary.PrintString` (`KismetStringLibrary.Concat_StrStr` "Error! " "The following material was not found in the Materials database: " (`|GetEnumeratorNameAsString` Material)) true true (struct :`G` 0.66 :`B` 1.0 :`A` 1.0) 10.0))))

(fn `UpdateTagVisibility`
  (params (Tag :type String) (Visibility :type String))
  ;[1 0.9609 0] Update Static Meshes with Tag to be visible or not according to Visibility
  (bind _outactors (`GameplayStatics.GetAllActorsOfClassWithTag` "/Script/Engine.StaticMeshActor" (`KismetStringLibrary.Conv_StringToName` Tag)))
  (if (== Visibility "True")
    (for _array_element _outactors
      (`SceneComponent.SetVisibility` (`Actor.RootComponent` _array_element) true true))
    (elif (== Visibility "False")
      (for _array_element_2 _outactors
        (`SceneComponent.SetVisibility` (`Actor.RootComponent` _array_element_2) false true))
      (else
        (`KismetSystemLibrary.PrintString` (`KismetStringLibrary.Concat_StrStr` "Error! " "The following Visibility Tag is not valid: " Visibility) true true (struct :`G` 0.66 :`B` 1.0 :`A` 1.0) 10.0)))))

(fn `UserConstructionScript`)