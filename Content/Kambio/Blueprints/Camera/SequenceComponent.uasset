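; Camera component that runs a looping, shuffled slideshow through level BP_CustomCamera actors, with fade transitions.
; RunSequencer disables rotation on every camera, shuffles those flagged WillBeInSequence and adds a fade widget to the viewport.
; Each cycle starts a ping-pong fade, switches the player's view target halfway through the fade duration, then holds for CameraDuration.
; Clearing SequenceIsRunning ends the loop after the current hold and removes the widget.
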(event `RunSequencer`
  (bind _returnvalue (`|CreateWidget` "/Game/Kambio/Blueprints/UI/Widgets/Transitions/Widget_FadeInOut.Widget_FadeInOut_C"))
  (`UserWidget.AddToViewport` _returnvalue 1)
  (set `self.WidgetFadeInOut` _returnvalue)
  (bind _outactors (`GameplayStatics.GetAllActorsOfClass` "/Game/Kambio/Blueprints/Camera/BP_CustomCamera.BP_CustomCamera_C"))
  (for _array_element _outactors
    (set `/Game/Kambio/Blueprints/Camera/BP_CustomCamera.CanRotate` false _array_element)
    (if (`/Game/Kambio/Blueprints/Camera/BP_CustomCamera.WillBeInSequence` _array_element)
      (`KismetArrayLibrary.Array_Add` (`self.CamerasForSequence`) _array_element)))
  (`KismetArrayLibrary.Array_Shuffle` (`self.CamerasForSequence`))
  (set `self.SequenceIsRunning` true)
  (`self.Fade in and Out` (`self.WidgetFadeInOut`) (`self.FadeDuration`) :!label _label)
  (`KismetSystemLibrary.Delay` (/ (`self.FadeDuration`) 2.0))
  (bind _output_get (set `self.CurrentCameraIdx` (mod (+ (`self.CurrentCameraIdx`) 1) (`KismetArrayLibrary.Array_Length` (`self.CamerasForSequence`)))))
  (`PlayerController.SetViewTargetWithBlend` (`GameplayStatics.GetPlayerController` 0) (`|GetArrayItem` (`self.CamerasForSequence`) _output_get) 0.0 "VTBlend_Linear" 0.0 false)
  (`KismetSystemLibrary.Delay` (`self.CameraDuration`))
  (if (`self.SequenceIsRunning`)
    (goto _label)
    (else
      (`Widget.RemoveFromParent` (`self.WidgetFadeInOut`)))))

(fn `Fade in and Out`
  (params (WidgetFadeInOut :type "/Game/Kambio/Blueprints/UI/Widgets/Transitions/Widget_FadeInOut Object Reference") (Duration :type "Float (double-precision)"))
  (locals (HalfDuration :type "Float (double-precision)"))
  (bind _output_get (set `local.HalfDuration` (/ Duration 2.0)))
  (`UserWidget.PlayAnimation` WidgetFadeInOut (`/Game/Kambio/Blueprints/UI/Widgets/Transitions/Widget_FadeInOut.Fade` WidgetFadeInOut) 0.0 1 "PingPong" (/ 1.0 _output_get) false))