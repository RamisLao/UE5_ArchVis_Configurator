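; Deprecated orbit camera actor that circles a target actor in response to horizontal look input from BP_KambioPlayerController.
; Input accumulates a rotation that places the actor on a radius around the target's Z axis, then turns it to face the target, with an optional debug line.
; The orbit uses a hardcoded angle offset; the starting angle computed at BeginPlay is passed in but unused.
; A helper can restore the initial location.
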(event `self.ReceiveBeginPlay`
  (set `self.InitialLocation` (`self.K2_GetActorLocation`))
  (bind _angle (`self.CalculateInitialAngle`))
  (bind _output_get (set `self.StartingAngle` _angle))
  (`KismetSystemLibrary.PrintString` (`KismetStringLibrary.Conv_DoubleToString` _output_get) false false)
  (bind _asbp_kambio_player_controller (cast `/Game/Kambio/Blueprints/Player/BP_KambioPlayerController` (`GameplayStatics.GetPlayerController` 0)))
  (add `/Game/Kambio/Blueprints/Player/BP_KambioPlayerController.EventLookHorizontal` _asbp_kambio_player_controller (delegate `OnLookHorizontal`))
  (set `self.CurrentRotation` (+ (`self.CurrentRotation`) (* (* (`self.RotationSpeed`) (stale `self.ReceiveTick` DeltaSeconds)) (stale `OnLookHorizontal` Value))) :!label _label)
  (`self.RotateActorAroundPoint` self (`self.TargetActor`) (`self.Radius`) (`self.StartingAngle`) (`self.CurrentRotation`))
  (`self.K2_SetActorRotation` (`KismetMathLibrary.FindLookAtRotation` (`self.K2_GetActorLocation`) (`self.K2_GetActorLocation` (`self.TargetActor`))))
  (if (`self.DrawDebug`)
    (`KismetSystemLibrary.DrawDebugLine` (`self.K2_GetActorLocation` (`self.TargetActor`)) (`self.K2_GetActorLocation`) (`self.TraceColor`) 1.0 2.0)))

(event `OnLookHorizontal`
  (params (Value :type "Float (double-precision)"))
  (goto _label))

(event `self.ReceiveTick`
  (params (DeltaSeconds :type "Float (single-precision)")))

(fn `CalculateInitialAngle`
  (returns (Angle :type "Float (double-precision)"))
  (return (`KismetMathLibrary.DegAcos` (`KismetMathLibrary.Dot_VectorVector` (`KismetMathLibrary.Normal` (`self.K2_GetActorLocation`)) (1.0 0.0 0.0)))))

(fn `ReturnToInitialPosition`
  ;[0 1 0.3203] Return actor to the original location
  (`self.K2_SetActorLocation` (`self.InitialLocation`)))

(fn `RotateActorAroundPoint`
  (params (ActorToRotate :type "Actor Object Reference") (TargetActor :type "Actor Object Reference") (Radius :type "Float (double-precision)") (Angle :type "Float (double-precision)") (RotationRate :type "Float (double-precision)"))
  (locals (LActorToRotate :type "Actor Object Reference") (LTargetActor :type "Actor Object Reference") (LTargetLocation :type "Vector Structure") (LRadius :type "Float (double-precision)") (LAngle :type "Float (double-precision)") (LRotationRate :type "Float (double-precision)"))
  (bind (_returnvalue_x _returnvalue_y _returnvalue_z) (`KismetMathLibrary.BreakVector` (`self.K2_GetActorLocation`)))
  (bind _ltargetactor (`local.LTargetActor`))
  (set `local.LRotationRate` RotationRate)
  (set `local.LAngle` Angle)
  (set `local.LRadius` Radius)
  (set `local.LTargetActor` TargetActor)
  (set `local.LActorToRotate` ActorToRotate)
  (`/Engine/EditorBlueprintResources/StandardMacros.IsValid` _ltargetactor
    (:`Is Valid`
      (`self.K2_SetActorLocation` (`local.LActorToRotate`) (+ (`self.K2_GetActorLocation` _ltargetactor) (`KismetMathLibrary.RotateAngleAxis` (`KismetMathLibrary.MakeVector` (`local.LRadius`) 0.0 _returnvalue_z) (+ -130.0 (`local.LRotationRate`)) (0.0 0.0 1.0))) false false)
      (return))))

(fn `UserConstructionScript`)