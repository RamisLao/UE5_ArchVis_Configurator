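; BP_CameraManager switches the player's view between two placed cameras and the player character.
; On BeginPlay it binds to the Pressed1, Pressed2 and PressedE events of BP_KambioPlayerController.
; Each handler calls SetNewViewTarget, which blends the player controller's view to Camera1, Camera2 or the player character over the BlendSpeed time.
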(event `self.ReceiveBeginPlay`
  (bind _asbp_kambio_player_controller (cast `/Game/Kambio/Blueprints/Player/BP_KambioPlayerController` (`GameplayStatics.GetPlayerController` 0)))
  (add `/Game/Kambio/Blueprints/Player/BP_KambioPlayerController.EventPressed1` _asbp_kambio_player_controller (delegate `Pressed 1`))
  (add `/Game/Kambio/Blueprints/Player/BP_KambioPlayerController.EventPressed2` _asbp_kambio_player_controller (delegate `Pressed 2`))
  (add `/Game/Kambio/Blueprints/Player/BP_KambioPlayerController.EventPressedE` _asbp_kambio_player_controller (delegate `Pressed E`)))

(event `Pressed 1`
  (`self.SetNewViewTarget` (`self.Camera 1`)))

(event `Pressed 2`
  (`self.SetNewViewTarget` (`self.Camera 2`)))

(event `Pressed E`
  (`self.SetNewViewTarget` (`GameplayStatics.GetPlayerCharacter` 0)))

(fn `SetNewViewTarget`
  (params (NewViewTarget :type "Actor Object Reference"))
  (`PlayerController.SetViewTargetWithBlend` (`GameplayStatics.GetPlayerController` 0) NewViewTarget (`self.BlendSpeed`) "VTBlend_Linear" 0.0 false))

(fn `UserConstructionScript`)