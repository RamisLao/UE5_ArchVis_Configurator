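; BP_CustomCamera is a camera node linked to up to four neighbor cameras (forward, right, back, left), with a ground arrow pointing toward one during exploration.
; BeginPlay collects valid neighbors; while active and exploring, Tick line-traces from the camera through the mouse to place the arrow, enlarging it as hit distance shrinks.
; The arrow yaws toward the neighbor with the smallest angle to the camera's forward vector, or hides when none exist.
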(event `self.ReceiveBeginPlay`
  (bind _cameraarray (`self.CameraArray`))
  (bind _cameraforward (`self.CameraForward`))
  (bind _cameraright (`self.CameraRight`))
  (bind _cameraback (`self.CameraBack`))
  (bind _cameraleft (`self.CameraLeft`))
  (`parent.ReceiveBeginPlay`)
  (`/Engine/EditorBlueprintResources/StandardMacros.IsValid` _cameraforward
    (:`Is Valid`
      (`KismetArrayLibrary.Array_Add` _cameraarray _cameraforward))
    (:`Is Not Valid`
      _))
  (`/Engine/EditorBlueprintResources/StandardMacros.IsValid` _cameraright
    (:`Is Valid`
      (`KismetArrayLibrary.Array_Add` _cameraarray _cameraright))
    (:`Is Not Valid`
      _))
  (`/Engine/EditorBlueprintResources/StandardMacros.IsValid` _cameraback
    (:`Is Valid`
      (`KismetArrayLibrary.Array_Add` _cameraarray _cameraback))
    (:`Is Not Valid`
      _))
  (`/Engine/EditorBlueprintResources/StandardMacros.IsValid` _cameraleft
    (:`Is Valid`
      (`KismetArrayLibrary.Array_Add` _cameraarray _cameraleft))))

(event `self.ReceiveTick`
  (params (DeltaSeconds :type "Float (single-precision)"))
  (bind _planearrow (`self.PlaneArrow`))
  (bind _cameracomponent (`self.CameraComponent`))
  (bind _planearrow_2 (`self.PlaneArrow`))
  (bind _da_configgameplay (`self.DA_ConfigGameplay`))
  (bind _returnvalue (`SceneComponent.K2_GetComponentLocation` (`self.CameraComponent`)))
  (bind _z (.z (`SceneComponent.K2_GetComponentLocation` _planearrow)))
  (if (`self.IsActive`)
    (if (`self.IsExploring`)
      (if (> (`KismetArrayLibrary.Array_Length` (`self.CameraArray`)) 0)
        (bind _outhit (`KismetSystemLibrary.LineTraceSingle` :`Start` _returnvalue :`End` (+ (* (`KismetMathLibrary.Normal` (- (`PlayerController.DeprojectMousePositionToWorld` (`GameplayStatics.GetPlayerController` 0)) _returnvalue)) (`/Game/Kambio/DataAssets/Config/PDAs/PDA_ConfigGameplay.LineTraceGroundLength` (`self.DA_ConfigGameplay`))) _returnvalue) :`TraceChannel` "TraceTypeQuery4" :`TraceColor` (struct :`R` 0.953019 :`B` 1.0 :`A` 1.0) :`TraceHitColor` (struct :`G` 0.000306 :`B` 1.0 :`A` 1.0) :`DrawTime` 2.0))
        (bind (_bblockinghit _binitialoverlap _time _distance _location) (`GameplayStatics.BreakHitResult` _outhit))
        (`SceneComponent.K2_SetWorldLocation` _planearrow_2 _location false false)
        (`SceneComponent.SetWorldScale3D` _planearrow_2 (`KismetMathLibrary.Conv_DoubleToVector` (`self.Denormalize` (- 1.0 (`self.Normalize` _distance 0.0 (`/Game/Kambio/DataAssets/Config/PDAs/PDA_ConfigGameplay.LineTraceGroundLength` (`self.DA_ConfigGameplay`)))) (`/Game/Kambio/DataAssets/Config/PDAs/PDA_ConfigGameplay.MinMoveArrowLength` _da_configgameplay) (`/Game/Kambio/DataAssets/Config/PDAs/PDA_ConfigGameplay.MaxMoveArrowLength` _da_configgameplay))))
        (set `self.SmallestAngleToCamera` 1000.0)
        (for _array_element (`self.CameraArray`)
          (bind _returnvalue_2 (`KismetMathLibrary.DegAcos` (`KismetMathLibrary.Dot_VectorVector` (`SceneComponent.GetForwardVector` _cameracomponent) (`KismetMathLibrary.Normal` (- (`SceneComponent.K2_GetComponentLocation` (`CameraActor.CameraComponent` _array_element)) (`SceneComponent.K2_GetComponentLocation` _cameracomponent))))))
          (if (< _returnvalue_2 (`self.SmallestAngleToCamera`))
            (set `self.SmallestAngleToCamera` _returnvalue_2)
            (set `self.CameraWithSmallestAngle` _array_element)))
        (`SceneComponent.K2_SetWorldRotation` _planearrow (`KismetMathLibrary.FindLookAtRotation` (`KismetMathLibrary.MakeVector` (.x (`SceneComponent.K2_GetComponentLocation` (`self.CameraComponent`))) (.y (`SceneComponent.K2_GetComponentLocation` (`self.CameraComponent`))) _z) (`KismetMathLibrary.MakeVector` (.x (`SceneComponent.K2_GetComponentLocation` (`CameraActor.CameraComponent` (`self.CameraWithSmallestAngle`)))) (.y (`SceneComponent.K2_GetComponentLocation` (`CameraActor.CameraComponent` (`self.CameraWithSmallestAngle`)))) _z)) false false)
        (else
          (`self.HideArrow`))))))

(fn `HideArrow`
  (if (`self.ArrowIsVisible`)
    (`SceneComponent.SetVisibility` (`self.PlaneArrow`) false false)
    (set `self.ArrowIsVisible` false)))

(fn `ReturnToInitialSetup`)

(fn `ShowArrow`
  (if (not (`self.ArrowIsVisible`))
    (`SceneComponent.SetVisibility` (`self.PlaneArrow`) true false)
    (set `self.ArrowIsVisible` true)))

(fn `UserConstructionScript`)