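; BP_StaticCamera is a camera that stays in place and lets the player rotate its view when rotation is allowed.
; On BeginPlay it stores the initial rotation and binds to the horizontal and vertical look events of BP_KambioPlayerController.
; Look input, scaled by rotation speed, adds relative yaw or inverted pitch to the camera component, without delta-time scaling.
; Its ReturnToInitialSetup extends the parent version by restoring the stored rotation.
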(event `self.ReceiveBeginPlay`
  ;[0.007812 1 0] Setup camera initial state and bind events
  (set `self.InitialRotation` (`SceneComponent.RelativeRotation` (`self.CameraComponent`)))
  (bind _asbp_kambio_player_controller (cast `/Game/Kambio/Blueprints/Player/BP_KambioPlayerController` (`GameplayStatics.GetPlayerController` 0)))
  (add `/Game/Kambio/Blueprints/Player/BP_KambioPlayerController.EventLookHorizontal` _asbp_kambio_player_controller (delegate `OnLookHorizontal`))
  (add `/Game/Kambio/Blueprints/Player/BP_KambioPlayerController.EventLookVertical` _asbp_kambio_player_controller (delegate `OnLookVertical`)))

(event `OnLookHorizontal`
  (params (Value :type "Float (double-precision)"))
  ;[1 0.1406 0] Rotate Camera horizontally
  (if (`self.CanRotate`)
    (`SceneComponent.K2_AddRelativeRotation` (`self.CameraComponent`) (`KismetMathLibrary.MakeRotator` 0.0 0.0 (* Value (`self.RotationSpeed`))) false false)))

(event `OnLookVertical`
  (params (Value :type "Float (double-precision)"))
  ;[0.5 0 1] Rotate Camera vertically
  (if (`self.CanRotate`)
    (`SceneComponent.K2_AddRelativeRotation` (`self.CameraComponent`) (`KismetMathLibrary.MakeRotator` 0.0 (* (* Value (`self.RotationSpeed`)) -1.0)) false false)))

(fn `ReturnToInitialRotation`
  ;[0.2891 1 0] Return camera to its original rotation
  (`SceneComponent.K2_SetRelativeRotation` (`self.CameraComponent`) (`self.InitialRotation`) false false))

(fn `ReturnToInitialSetup`
  (`parent.ReturnToInitialSetup`)
  (`self.ReturnToInitialRotation`))

(fn `UserConstructionScript`)