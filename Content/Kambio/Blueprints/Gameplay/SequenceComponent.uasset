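; Component that runs a looping cinematic camera sequence, cycling the player's view through flagged BP_CustomCamera actors in shuffled order.
; RunSequencer disables rotation on all such cameras, then repeatedly starts a ping-pong fade, switches view target after half the fade duration and holds each shot until SequenceIsRunning clears.
; Helpers create, play and remove the fade widget, which is added to the viewport only when created opaque, unlike in RunSequencer.
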(event `RunSequencer`
  (`self.CreateWidgetFade` false)
  (bind _outactors (`GameplayStatics.GetAllActorsOfClass` "/Game/Kambio/Blueprints/Camera/BP_CustomCamera.BP_CustomCamera_C"))
  (for _array_element _outactors
    (set `/Game/Kambio/Blueprints/Camera/BP_CustomCamera.CanRotate` false _array_element)
    (if (`/Game/Kambio/Blueprints/Camera/BP_CustomCamera.WillBeInSequence` _array_element)
      (`KismetArrayLibrary.Array_Add` (`self.CamerasForSequence`) _array_element)))
  (`KismetArrayLibrary.Array_Shuffle` (`self.CamerasForSequence`))
  (set `self.SequenceIsRunning` true)
  (`self.FadeInAndOut` (`self.WidgetFadeInOut`) (`self.FadeDuration`) :!label _label)
  (`KismetSystemLibrary.Delay` (/ (`self.FadeDuration`) 2.0))
  (bind _output_get (set `self.CurrentCameraIdx` (mod (+ (`self.CurrentCameraIdx`) 1) (`KismetArrayLibrary.Array_Length` (`self.CamerasForSequence`)))))
  (`PlayerController.SetViewTargetWithBlend` (`GameplayStatics.GetPlayerController` 0) (`|GetArrayItem` (`self.CamerasForSequence`) _output_get) 0.0 "VTBlend_Linear" 0.0 false)
  (`KismetSystemLibrary.Delay` (`self.CameraDuration`))
  (if (`self.SequenceIsRunning`)
    (goto _label)
    (else
      (`self.DestroyWidgetFade`))))

(fn `CreateWidgetFade`
  (params (StartOpaque :type Boolean))
  (bind _returnvalue (`|CreateWidget` "/Game/Kambio/Blueprints/UI/Widgets/Transitions/Widget_FadeInOut.Widget_FadeInOut_C"))
  (bind _output_get (set `self.WidgetFadeInOut` _returnvalue))
  (if StartOpaque
    (bind _border (`/Game/Kambio/Blueprints/UI/Widgets/Transitions/Widget_FadeInOut.Border` _output_get))
    (`Border.SetBrushColor` _border (struct :`A` 1.0))
    (`UserWidget.AddToViewport` _returnvalue 1)
    (else
      (`Border.SetBrushColor` :`self` _border))))

(fn `DestroyWidgetFade`
  (bind _widgetfadeinout (`self.WidgetFadeInOut`))
  (`/Engine/EditorBlueprintResources/StandardMacros.IsValid` _widgetfadeinout
    (:`Is Valid`
      (`Widget.RemoveFromParent` _widgetfadeinout))))

(fn `FadeIn`
  (bind _widgetfadeinout (`self.WidgetFadeInOut`))
  (`/Engine/EditorBlueprintResources/StandardMacros.IsValid` _widgetfadeinout
    (:`Is Valid`
      (`UserWidget.PlayAnimation` _widgetfadeinout (`/Game/Kambio/Blueprints/UI/Widgets/Transitions/Widget_FadeInOut.Fade` _widgetfadeinout) 0.0 1 "Forward" 1.0 false))))

(fn `FadeInAndOut`
  (params (WidgetFadeInOut :type "/Game/Kambio/Blueprints/UI/Widgets/Transitions/Widget_FadeInOut Object Reference") (Duration :type "Float (double-precision)"))
  (locals (DoubleDuration :type "Float (double-precision)"))
  (bind _output_get (set `local.DoubleDuration` (* Duration 2.0)))
  (`UserWidget.PlayAnimation` WidgetFadeInOut (`/Game/Kambio/Blueprints/UI/Widgets/Transitions/Widget_FadeInOut.Fade` WidgetFadeInOut) 0.0 1 "PingPong" (/ 1.0 _output_get) false))

(fn `FadeOut`
  (bind _widgetfadeinout (`self.WidgetFadeInOut`))
  (`/Engine/EditorBlueprintResources/StandardMacros.IsValid` _widgetfadeinout
    (:`Is Valid`
      (`UserWidget.PlayAnimation` _widgetfadeinout (`/Game/Kambio/Blueprints/UI/Widgets/Transitions/Widget_FadeInOut.Fade` _widgetfadeinout) 0.0 1 "Reverse" 1.0 false))))