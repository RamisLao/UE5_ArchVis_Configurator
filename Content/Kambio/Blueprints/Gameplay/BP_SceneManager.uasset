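; BP_SceneManager chooses which level to load from the modelId parameter on the game's command line.
; On BeginPlay it stores the command line in CommandLineInput and checks it for modelId.
; When present, it parses the value, strips the equals sign and looks it up in the ModelIdToLevel map.
; It prints the mapped level name and loads it as a level instance, without checking that the lookup succeeded.
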(event `self.ReceiveBeginPlay`
  (bind _value (`BlueprintMapLibrary.Map_Find` (`/Game/Kambio/Blueprints/DataAssets/PDA_ModelIdToLevel.ModelIdToLevel` (`self.ModelIdToLevel`)) (`KismetStringLibrary.Replace` (`KismetSystemLibrary.ParseParamValue` (`/Game/Kambio/Blueprints/DataAssets/PDA_CommandLineInput.Input` (`self.CommandLineInput`)) "modelId") "=")))
  (bind _returnvalue (`KismetSystemLibrary.GetCommandLine`))
  (set `/Game/Kambio/Blueprints/DataAssets/PDA_CommandLineInput.Input` _returnvalue (`self.CommandLineInput`))
  (if (`KismetStringLibrary.Contains` (`/Game/Kambio/Blueprints/DataAssets/PDA_CommandLineInput.Input` (`self.CommandLineInput`)) "modelId")
    (`KismetSystemLibrary.PrintString` _value)
    (`LevelStreamingDynamic.LoadLevelInstance` _value (0.0 0.0 0.0) (struct) "" null)))

(fn `UserConstructionScript`)