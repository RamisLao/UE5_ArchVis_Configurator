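; Player controller for an app that switches between Configuration, Exploration and Cinematics modes, each with its own HUD.
; CameraManager, UIConfig and Sequence components handle cameras, panels and sequences; startup fades into Configuration.
; Mouse and touch share press/release logic: drag rotates the view, short taps in Exploration change camera, release in Cinematics returns to Configuration.
; Throttled wheel input scrolls UI panels, panel changes update the configuration camera, and Pixel Streaming input is printed.
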(event `Key|LeftMouseButton`
  (params (Key :type "Key Structure"))
  ;[1 0.9141 0] Input
  (:`Pressed`
    (if (`|EnumEquality` (`self.CurrentAppMode`) "NewEnumerator1") :!label _label
      (set `self.TimeSinceLeftMousePressed` 0.0)
      (elif (`self.CanActivateCameraRotation`)
        (set `self.CanRotateCamera` true))))
  (:`Released`
    (switch `/Game/Kambio/Enums/Enum_AppMode` (`self.CurrentAppMode`) :!label _label_2
      (:`NewEnumerator0`
        (if (`self.CanActivateCameraRotation`)
          (set `self.CanRotateCamera` false)))
      (:`NewEnumerator1`
        (if (< (`self.TimeSinceLeftMousePressed`) (`self.DelayThresholdToChangeCamera`))
          (`/Game/Kambio/Blueprints/Components/CameraManagerComponent.SetNewCameraForExploration` (`self.CameraManagerComponent`))))
      (:`NewEnumerator2`
        (`self.GoToConfigurationMode`)))))

(event `self.ReceiveBeginPlay`
  (bind _uiconfigcomponent (`self.UIConfigComponent`))
  ;[0 0.4609 1] Setup
  (`/Game/Kambio/Blueprints/Components/SequenceComponent.CreateWidgetFade` (`self.SequenceComponent`) true)
  (set `self.bShowMouseCursor` true)
  (set `self.CanActivateCameraRotation` false)
  (set `self.CanRotateCamera` false)
  (bind _outactors (`GameplayStatics.GetAllActorsOfClass` "/Game/Kambio/Blueprints/Cameras/BP_MapCamera.BP_MapCamera_C"))
  (set `/Game/Kambio/Blueprints/Components/CameraManagerComponent.MapCamera` (`|GetArrayItem` _outactors) (`self.CameraManagerComponent`))
  (add `PixelStreamingInput.OnInputEvent` (`self.PixelStreamingInput`) (delegate `OnPixelStreamingInputEvent`))
  (add `/Game/Kambio/Blueprints/Components/Component_UIConfig.OnActiveWidgetPanelChanged` _uiconfigcomponent (delegate `OnActiveWidgetPanelChanged`))
  (add `/Game/Kambio/Blueprints/Components/Component_UIConfig.OnButtonConfigurationClicked` _uiconfigcomponent (`|CreateDelegate` :!event `GoToConfigurationMode`))
  (add `/Game/Kambio/Blueprints/Components/Component_UIConfig.OnButtonExplorationClicked` _uiconfigcomponent (`|CreateDelegate` :!event `GoToExplorationMode`))
  (add `/Game/Kambio/Blueprints/Components/Component_UIConfig.OnButtonCinematicsClicked` _uiconfigcomponent (`|CreateDelegate` :!event `GoToCinematicMode`))
  (bind _outactors_2 (`GameplayStatics.GetAllActorsOfClassWithTag` "/Game/Kambio/Blueprints/Cameras/BP_CustomCamera.BP_CustomCamera_C" (`KismetStringLibrary.Conv_StringToName` (`/Game/Kambio/DataAssets/PDAs/PDA_ConfigGameplay.InitCameraTagForExploration` (`self.DA_ConfigGameplay`)))))
  (`/Game/Kambio/Blueprints/Components/CameraManagerComponent.Set New Camera` (`self.CameraManagerComponent`) (`|GetArrayItem` _outactors_2) false false 1.0)
  (`KismetSystemLibrary.Delay` 0.5)
  (`/Game/Kambio/Blueprints/Components/SequenceComponent.FadeOut` (`self.SequenceComponent`))
  (`KismetSystemLibrary.Delay` 1.5)
  (`/Game/Kambio/Blueprints/Components/SequenceComponent.DestroyWidgetFade` (`self.SequenceComponent`))
  (`self.GoToConfigurationMode`))

(event `InputTouch`
  (params (Location :type "Vector Structure") (FingerIndex :type "ETouchIndex Enum"))
  ;[1 0.9141 0] Input
  (:`Pressed`
    (set `self.LastTouchedLocation` Location)
    (goto _label))
  (:`Released`
    (goto _label_2)))

(event `OnPixelStreamingInputEvent`
  (params (Descriptor :type String))
  (bind (_stringvalue _success) (`PixelStreamingInput.GetJsonStringValue` (`self.PixelStreamingInput`) Descriptor ""))
  ;[0 0.4609 1] Setup
  (if _success
    (`KismetSystemLibrary.PrintString` _stringvalue)))

(event `InputAxis|LookHorizontal`
  (params (AxisValue :type "Float (single-precision)"))
  ;[1 0.9141 0] Input
  (if (`self.CanRotateCamera`)
    (`self.RotateHorizontally` AxisValue)))

(event `OnActiveWidgetPanelChanged`
  (params (ActiveSwitcherPanel :type "/Game/Kambio/Blueprints/UI/Widgets/Panels/Widget_SwitcherPanel Object Reference") (ResetCamera :type Boolean))
  ;[0 0.4609 1] Setup
  (`/Game/Kambio/Blueprints/Components/CameraManagerComponent.SetNewCameraForConfiguration` (`self.CameraManagerComponent`) ActiveSwitcherPanel ResetCamera))

(event `InputTouch`
  (params (Location :type "Vector Structure") (FingerIndex :type "ETouchIndex Enum"))
  ;[1 0.9141 0] Input
  (:`Moved`
    (if (`self.CanRotateCamera`)
      (`self.RotateHorizontally` (* (`KismetMathLibrary.FClamp` (- (.x Location) (.x (`self.LastTouchedLocation`))) -1.0) 0.2)))))

(event `self.ReceiveTick`
  (params (DeltaSeconds :type "Float (single-precision)"))
  ;[0 0.8359 1] Tick
  (set `self.TimeSinceLastScroll` (+ (`self.TimeSinceLastScroll`) DeltaSeconds))
  (set `self.TimeSinceLeftMousePressed` (+ (`self.TimeSinceLeftMousePressed`) DeltaSeconds)))

(event `InputAxis|LookVertical`
  (params (AxisValue :type "Float (single-precision)"))
  ;[1 0.9141 0] Input
  (if (`self.CanRotateCamera`)
    (`self.RotateVertically` AxisValue)))

(event `InputTouch`
  (params (Location :type "Vector Structure") (FingerIndex :type "ETouchIndex Enum"))
  ;[1 0.9141 0] Input
  (:`Moved`
    (if (`self.CanRotateCamera`)
      (`self.RotateVertically` (* (`KismetMathLibrary.FClamp` (- (.y Location) (.y (`self.LastTouchedLocation`))) -1.0) -1.0 0.2))
      (set `self.LastTouchedLocation` Location))))

(event `InputAction|MouseWheelUp`
  (params (Key :type "Key Structure"))
  ;[1 0.9141 0] Input
  (:`Pressed`
    (if (>= (`self.TimeSinceLastScroll`) (`self.DelayBetweenScrolling`))
      (`/Game/Kambio/Blueprints/Components/Component_UIConfig.MaybeScrollToLastSwitcherPanel` (`self.UIConfigComponent`))
      (set `self.TimeSinceLastScroll` 0.0 :!label _label_3))))

(event `InputAction|MouseWheelDown`
  (params (Key :type "Key Structure"))
  ;[1 0.9141 0] Input
  (:`Pressed`
    (if (>= (`self.TimeSinceLastScroll`) (`self.DelayBetweenScrolling`))
      (`/Game/Kambio/Blueprints/Components/Component_UIConfig.MaybeScrollToNextSwitcherPanel` (`self.UIConfigComponent`))
      (goto _label_3))))

(fn `GoToCinematicMode`
  (if (not (`|EnumEquality` (`self.CurrentAppMode`) "NewEnumerator2"))
    (`/Game/Kambio/Blueprints/Cameras/BP_CustomCamera.HideViewPlane` (`/Game/Kambio/Blueprints/Components/CameraManagerComponent.CurrentCamera` (`self.CameraManagerComponent`)))
    (set `self.CurrentAppMode` "NewEnumerator2")
    (`/Game/Kambio/Blueprints/Components/Component_UIConfig.InstantiateHUDSmall` (`self.UIConfigComponent`) "NewEnumerator2")
    (`/Game/Kambio/Blueprints/Components/SequenceComponent.RunSequencer` (`self.SequenceComponent`))))

(fn `GoToConfigurationMode`
  (bind _currentcamera (`/Game/Kambio/Blueprints/Components/CameraManagerComponent.CurrentCamera` (`self.CameraManagerComponent`)))
  (if (not (`|EnumEquality` (`self.CurrentAppMode`) "NewEnumerator0"))
    (set `/Game/Kambio/Blueprints/Components/SequenceComponent.SequenceIsRunning` false (`self.SequenceComponent`))
    (`/Engine/EditorBlueprintResources/StandardMacros.IsValid` _currentcamera
      (:`Is Valid`
        (set `/Game/Kambio/Blueprints/Cameras/BP_CustomCamera.IsExploring` false _currentcamera))
      (:`Is Not Valid`
        _))
    (set `self.CurrentAppMode` "NewEnumerator0")
    (`/Game/Kambio/Blueprints/Components/Component_UIConfig.InstantiateHUD` (`self.UIConfigComponent`))
    (set `self.CanActivateCameraRotation` true)))

(fn `GoToExplorationMode`
  (if (not (`|EnumEquality` (`self.CurrentAppMode`) "NewEnumerator1"))
    (`/Game/Kambio/Blueprints/Cameras/BP_CustomCamera.HideViewPlane` (`/Game/Kambio/Blueprints/Components/CameraManagerComponent.CurrentCamera` (`self.CameraManagerComponent`)))
    (set `/Game/Kambio/Blueprints/Components/SequenceComponent.SequenceIsRunning` false (`self.SequenceComponent`))
    (bind _outactors (`GameplayStatics.GetAllActorsOfClassWithTag` "/Game/Kambio/Blueprints/Cameras/BP_CustomCamera.BP_CustomCamera_C" (`KismetStringLibrary.Conv_StringToName` (`/Game/Kambio/DataAssets/PDAs/PDA_ConfigGameplay.InitCameraTagForExploration` (`self.DA_ConfigGameplay`)))))
    (bind _output_get (set `/Game/Kambio/Blueprints/Components/CameraManagerComponent.CurrentCamera` (`|GetArrayItem` _outactors) (`self.CameraManagerComponent`)))
    (set `/Game/Kambio/Blueprints/Cameras/BP_CustomCamera.IsExploring` true _output_get)
    (`/Game/Kambio/Blueprints/Cameras/BP_CustomCamera.ShowArrow` _output_get)
    (`/Game/Kambio/Blueprints/Components/CameraManagerComponent.Set New Camera` (`self.CameraManagerComponent`) _output_get false false 1.0)
    (set `self.CanRotateCamera` true)
    (set `self.CurrentAppMode` "NewEnumerator1")
    (`/Game/Kambio/Blueprints/Components/Component_UIConfig.InstantiateHUDSmall` (`self.UIConfigComponent`) "NewEnumerator1")))

(fn `RotateHorizontally`
  (params (AxisValue :type "Float (double-precision)"))
  (bind _returnvalue (* AxisValue (`GameplayStatics.GetWorldDeltaSeconds`) (`self.RotationSpeed`) -1.0))
  ;[0.4766 1 0] Rotate current character horizontally and call event LookHorizontal
  (`Pawn.AddControllerYawInput` (`GameplayStatics.GetPlayerCharacter` 0) _returnvalue)
  (`self.EventLookHorizontal` _returnvalue))

(fn `RotateVertically`
  (params (AxisValue :type "Float (double-precision)"))
  (bind _returnvalue (* AxisValue (`GameplayStatics.GetWorldDeltaSeconds`) (`self.RotationSpeed`)))
  ;[0.9922 0 1] Rotate current character vertically and send event LookVertical
  (`Pawn.AddControllerPitchInput` (`GameplayStatics.GetPlayerCharacter` 0) _returnvalue)
  (`self.EventLookVertical` _returnvalue))

(fn `UserConstructionScript`)