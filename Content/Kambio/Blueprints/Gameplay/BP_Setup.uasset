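; Startup Blueprint that picks which level to stream in from a modelId command-line argument.
; On BeginPlay it stores the command line in the DACommandLineInput data asset and checks it for modelId.
; The parsed value, stripped of "=", is looked up in the DAModelIdToLevel map, and the resulting level name is printed and loaded as a level instance.
; LoadScene and ParseUrlParams are empty stubs.
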(event `self.ReceiveBeginPlay`
  (bind _value (`BlueprintMapLibrary.Map_Find` (`/Game/Kambio/DataAssets/Config/PDAs/PDA_ModelIdToLevel.ModelIdToLevel` (`self.DA_ModelIdToLevel`)) (`KismetStringLibrary.Replace` (`KismetSystemLibrary.ParseParamValue` (`/Game/Kambio/DataAssets/Config/PDAs/PDA_CommandLineInput.Input` (`self.DA_CommandLineInput`)) "modelId") "=")))
  (bind _returnvalue (`KismetSystemLibrary.GetCommandLine`))
  (set `/Game/Kambio/DataAssets/Config/PDAs/PDA_CommandLineInput.Input` _returnvalue (`self.DA_CommandLineInput`))
  (if (`KismetStringLibrary.Contains` (`/Game/Kambio/DataAssets/Config/PDAs/PDA_CommandLineInput.Input` (`self.DA_CommandLineInput`)) "modelId")
    (`KismetSystemLibrary.PrintString` _value)
    (`LevelStreamingDynamic.LoadLevelInstance` _value (0.0 0.0 0.0) (struct) "" null)))

(fn `LoadScene`)

(fn `ParseUrlParams`)

(fn `UserConstructionScript`)